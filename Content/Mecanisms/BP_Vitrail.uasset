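; BP_Vitrail is a stained-glass actor, apparently a grid-based sliding piece mechanism, still unfinished.
; On BeginPlay it converts the relative X and Z of each direct ControlRig child into a flat index, using 50-unit cells and Imax as row stride.
; It marks those cells occupied in the ListePieces boolean array.
; The four directional MovePiece events are empty stubs.
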(event Custom|MovePieceRight)

(event Custom|MovePieceLeft)

(event Custom|MovePieceUp)

(event Custom|MovePieceDown)

(event EventBeginPlay
  (for _array_element (Components|GetChildrenComponents (Variables|Default|GetControlRig) false)
    (Utilities|Array|SetArrayElem (Variables|Default|GetListePieces) (Math|Float|Truncate (+ (/ (.x (Variables|/Script/Engine.SceneComponent|GetRelativeLocation _array_element)) 5e+01) (* (/ (.z (Variables|/Script/Engine.SceneComponent|GetRelativeLocation _array_element)) -5e+01) (Variables|Default|Getimax)))) true)))

(event Collision|EventActorBeginOverlap
  (params (OtherActor :type Actor%20Object%20Reference)))

(event EventTick
  (params (DeltaSeconds :type Float%20%28single-precision%29)))

(fn ConstructionScript)