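; BP_BreakableObject is a breakable actor that leaves a pickable key behind when broken.
; It adds the "Pickups" tag to itself on BeginPlay.
; Its BreakObject event spawns a BP_PickableKey slightly above its own transform, sets that key's MyPickup from its Key value, then destroys itself.
; The file contains no call to BreakObject, so the break is triggered from outside.
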(event Custom|BreakObject
  (bind _self self)
  (bind _returnvalue (Transformation|GetActorTransform _self))
  (bind _returnvalue_2 (Game|SpawnActorfromClass :Class "/Game/Mecanisms/BP_PickableKey.BP_PickableKey_C" :SpawnTransform (Math|Transform|MakeTransform (Math|Vector|MakeVector (.x (.location _returnvalue)) (.y (.location _returnvalue)) (+ (.z (.location _returnvalue)) 2e+01)) (.rotation _returnvalue) (.scale _returnvalue)) :CollisionHandlingOverride "Undefined" :TransformScaleMethod "MultiplyWithRoot" :Instigator 0))
  (Variables|/Game/Mecanisms/BP_PickableKey.BP_PickableKey_C|SetMy%20Pickup _returnvalue_2 (Variables|Default|GetKey))
  (Actor|DestroyActor))

(event EventBeginPlay
  (Utilities|Array|Add (Variables|Actor|GetTags self) "Pickups"))

(fn ConstructionScript)