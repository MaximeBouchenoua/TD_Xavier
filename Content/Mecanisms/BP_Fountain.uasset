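; BP_Fountain is a fountain mechanism that accepts a key and reveals a hidden actor, named as a devil spawn, in its place in the level.
; PlaceKey spawns a sapphire activation object at the Box component's transform, destroys the Box, prints a debug message and sets IsOpen.
; It then calls SpawnDevil, which destroys the referenced DespawnActor and unhides the pre-placed SpawnActor.
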(event Custom|Place%20Key
  (Game|SpawnActorfromClass "/Game/Mecanisms/BP_ActivationObject_Sapphire.BP_ActivationObject_Sapphire_C" (Transformation|GetWorldTransform (Variables|Default|GetBox)) "Undefined" "MultiplyWithRoot" 0 0 0)
  (Components|DestroyComponent (Variables|Default|GetBox))
  (Development|PrintString "J'ai posé le livre")
  (Variables|Default|SetIsOpen true)
  (CallFunction|SpawnDevil))

(event Custom|Spawn%20Devil
  (Actor|DestroyActor (Variables|Default|GetDespawn%20Actor))
  (Rendering|SetActorHiddenInGame (Variables|Default|GetSpawn%20Actor) false))

(fn ConstructionScript)