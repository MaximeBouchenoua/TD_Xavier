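; BP_Worktable is an interactable worktable that triggers the endgame sequence when the player uses it.
; On interaction it disables movement, the diary and HUD use, hides all HUDs, and blends the camera to the table.
; After a delay it shows the character's endgame HUD.
; Exiting the interaction restores movement and blends the view back to the character, leaving HUD and diary flags untouched.
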(event Custom|ObjectInteraction
  (bind _asbp_third_person_character (Utilities|Casting|CastToBP_ThirdPersonCharacter (Game|GetPlayerCharacter 0)))
  (Variables|/Game/ThirdPerson/Blueprints/BP_ThirdPersonCharacter.BP_ThirdPersonCharacter_C|SetCanMove _asbp_third_person_character false)
  (Variables|/Game/ThirdPerson/Blueprints/BP_ThirdPersonCharacter.BP_ThirdPersonCharacter_C|SetHasDiary _asbp_third_person_character false)
  (Variables|/Game/ThirdPerson/Blueprints/BP_ThirdPersonCharacter.BP_ThirdPersonCharacter_C|SetCan%20Use%20HUD _asbp_third_person_character false)
  (Default|HideAllHUDs _asbp_third_person_character)
  (Game|Player|SetViewTargetwithBlend (Game|GetPlayerController 0) self 1.0 "VTBlend_Linear" 0.0 false)
  (Utilities|FlowControl|Delay 5.0)
  (Default|EndgameHUD _asbp_third_person_character))

(event Custom|ExitInteraction
  (bind _asbp_third_person_character (Utilities|Casting|CastToBP_ThirdPersonCharacter (Game|GetPlayerCharacter 0)))
  (Variables|/Game/ThirdPerson/Blueprints/BP_ThirdPersonCharacter.BP_ThirdPersonCharacter_C|SetCanMove _asbp_third_person_character true)
  (Game|Player|SetViewTargetwithBlend (Game|GetPlayerController 0) _asbp_third_person_character 1.0 "VTBlend_Linear" 0.0 false))

(event EventBeginPlay)

(event Collision|EventActorBeginOverlap
  (params (OtherActor :type Actor%20Object%20Reference)))

(event EventTick
  (params (DeltaSeconds :type Float%20%28single-precision%29)))

(fn ConstructionScript)