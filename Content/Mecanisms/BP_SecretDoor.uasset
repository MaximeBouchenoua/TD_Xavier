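; BP_SecretDoor is a secret door actor that disappears once all of its linked key mechanisms are open.
; Every tick it loops over the KeyMecanisms array, sets Canact only if each entry reports IsOpen, and stops at the first closed one.
; When Canact is true, the door removes itself by destroying its actor rather than animating open.
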(event Custom|MecanismCheck
  (bind _array_element (Utilities|Array|ForEachLoopwithBreak (Variables|Default|GetKeyMecanisms) :!label _label)
    (:LoopBody
      (if (Variables|/Game/Mecanisms/BP_Bookshelf.BP_Bookshelf_C|GetIsOpen _array_element)
        (Variables|Default|Setcanact true)
        (else
          (Variables|Default|Setcanact false)
          (goto _label Break))))
    (:Completed
      (if (Variables|Default|Getcanact)
        (Actor|DestroyActor self)))))

(event EventTick
  (params (DeltaSeconds :type Float%20%28single-precision%29))
  (CallFunction|MecanismCheck))

(fn ConstructionScript)