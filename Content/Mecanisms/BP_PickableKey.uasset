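; BP_PickableKey is a key pickup that records itself in the player character's key array when collected.
; Its PickingUp function sets a Done flag, casts player 0's pawn to BP_ThirdPersonCharacter, and sets the Keys entry at this key's ID to true.
; Tick polls the Done flag and destroys the actor, even if the cast fails, since the flag is set first.
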(event EventTick
  (params (DeltaSeconds :type Float%20%28single-precision%29))
  (if (Variables|Default|GetDone)
    (Actor|DestroyActor)))

(fn ConstructionScript)

(fn PickingUp
  (Variables|Default|SetDone true)
  (bind _asbp_third_person_character (Utilities|Casting|CastToBP_ThirdPersonCharacter (Game|GetPlayerCharacter 0)))
  (Utilities|Array|SetArrayElem (Variables|/Game/ThirdPerson/Blueprints/BP_ThirdPersonCharacter.BP_ThirdPersonCharacter_C|GetKeys _asbp_third_person_character) (Variables|Default|GetID) true)
  (return))