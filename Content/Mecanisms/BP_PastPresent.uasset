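; BP_PastPresent is a room volume that switches between a past and a present version of its contents.
; Its switch event hides one object array and shows the other by toggling actor visibility only.
; When the third-person character enters the Box, it registers itself as the room to change on the character's DiaryHUD.
; An inside-area flag tracks overlap, and debug strings print on each change.
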(event OnComponentBeginOverlap(Box)
  (params (OverlappedComponent :type Primitive%20Component%20Object%20Reference) (OtherActor :type Actor%20Object%20Reference) (OtherComp :type Primitive%20Component%20Object%20Reference) (OtherBodyIndex :type Integer) (bFromSweep :type Boolean) (SweepResult :type Hit%20Result%20Structure%20%28by%20ref%29))
  (bind _asbp_third_person_character (Utilities|Casting|CastToBP_ThirdPersonCharacter OtherActor))
  (Variables|/Game/HUD/Menus/WBP_Diary.WBP_Diary_C|SetRoomToChange (Variables|/Game/ThirdPerson/Blueprints/BP_ThirdPersonCharacter.BP_ThirdPersonCharacter_C|GetDiary_HUD _asbp_third_person_character) self)
  (Variables|Default|SetInsideCorrect%20Area true)
  (Development|PrintString "Enter Zone" true true "(R=0.962442,G=1.000000,B=0.964752,A=1.000000)" 5.0))

(event OnComponentEndOverlap(Box)
  (params (OverlappedComponent :type Primitive%20Component%20Object%20Reference) (OtherActor :type Actor%20Object%20Reference) (OtherComp :type Primitive%20Component%20Object%20Reference) (OtherBodyIndex :type Integer))
  (Utilities|Casting|CastToBP_ThirdPersonCharacter OtherActor)
  (Variables|Default|SetInsideCorrect%20Area false)
  (Development|PrintString "Exit Zone" true true "(R=0.962442,G=1.000000,B=0.964752,A=1.000000)" 5.0))

(event Custom|Spawn%20Past%20or%20Present
  (params (Go%20to%20Past :type Boolean))
  (bind _output_get (Variables|Default|SetIsPast? Go%20to%20Past))
  (if _output_get
    (for _array_element (Variables|Default|GetPast%20Objects)
      (Rendering|SetActorHiddenInGame _array_element false))
    (for _array_element_2 (Variables|Default|GetPresent%20Objects)
      (Rendering|SetActorHiddenInGame _array_element_2 true))
    (Development|PrintString "FINITO PAST")
    (else
      (for _array_element_3 (Variables|Default|GetPresent%20Objects)
        (Rendering|SetActorHiddenInGame _array_element_3 false))
      (for _array_element_4 (Variables|Default|GetPast%20Objects)
        (Rendering|SetActorHiddenInGame _array_element_4 true))
      (Development|PrintString "FINITO PRESENT"))))

(fn ConstructionScript)